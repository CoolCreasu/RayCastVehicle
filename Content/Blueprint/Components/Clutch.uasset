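; Clutch component for a vehicle drivetrain simulation, computing the torque passed between engine and gearbox.
; Each physics update takes output shaft speed, engine speed and gear ratio, deriving slip that is zeroed in neutral.
; Engagement ramps in with engine RPM just above idle, acting as an automatic clutch.
; Torque scales with slip, engagement and stiffness, is clamped to an engine-based capacity, then smoothed by damping against the previous value.
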(event Custom|UpdatePhysic
  (params (OutputShaftVelocity :type Float%20%28single-precision%29) (EngineAngularVelocity :type Float%20%28single-precision%29) (GearboxRatio :type Float%20%28single-precision%29))
  (Variables|Default|SetClutchAngularVelocity OutputShaftVelocity)
  (Variables|Default|SetEngineAngularVelocity EngineAngularVelocity)
  (Variables|Default|SetGearboxRatio GearboxRatio)
  (CallFunction|GetClutchTorque))

(event EventBeginPlay
  (CallFunction|Initialization))

(event EventTick
  (params (DeltaSeconds :type Float%20%28single-precision%29)))

(fn GetClutchTorque
  (bind _clutchmaxtorque (Variables|Default|GetClutchMaxTorque))
  (Variables|Default|SetClutchSlip (* (- (Variables|Default|GetEngineAngularVelocity) (Variables|Default|GetClutchAngularVelocity)) (Math|Float|Sign(Float) (Math|Float|Absolute(Float) (Variables|Default|GetGearboxRatio)))))
  (Variables|Default|SetClutchLock (Math|Float|Min(Float) (+ (Math|Float|MapRangeClamped (* (Variables|Default|GetEngineAngularVelocity) (Variables|Default|GetRadToRPM)) 1e+03 1.3e+03 0.0 1.0) (Math|Conversions|ToFloat(Boolean) (== (Variables|Default|GetGearboxRatio) 0.0))) 1.0))
  (Variables|Default|SetClutchTorque (+ (Math|Float|Clamp(Float) (* (Variables|Default|GetClutchSlip) (Variables|Default|GetClutchLock) (Variables|Default|GetClutchStiffness)) (* _clutchmaxtorque -1.0) _clutchmaxtorque) (* (- (Variables|Default|GetClutchTorque) (Math|Float|Clamp(Float) (* (Variables|Default|GetClutchSlip) (Variables|Default|GetClutchLock) (Variables|Default|GetClutchStiffness)) (* _clutchmaxtorque -1.0) _clutchmaxtorque)) (Variables|Default|GetClutchDamping)))))

(fn Initialization
  (Variables|Default|SetRadToRPM (/ 6e+01 (* (Math|Trig|GetPI) 2.0)))
  (Variables|Default|SetClutchMaxTorque (* (Variables|Default|GetEngineMaxTorque) (Variables|Default|GetClutchCapacity))))