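; Gearbox component that models a vehicle's manual-style transmission with reverse, neutral and numbered forward gears.
; Shift events step the gear within its limits, zeroing the ratio and blocking further shifts during a timed delay.
; GetRatio then sets the new ratio and display label.
; Helper functions multiply by that ratio to convert torque to the output side and shaft velocity to the input side.
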(event Custom|ShiftGearUp
  (if (and (< (Variables|Default|GetGear) (Variables|Default|GetNumOfGears)) (Variables|Default|GetInGear))
    (Variables|Default|SetInGear false)
    (Variables|Default|SetRatio 0.0)
    (Variables|Default|SetGearText "--")
    (Utilities|FlowControl|Delay (Variables|Default|GetGearShiftTime))
    (Variables|Default|SetInGear true)
    (Math|Integer|IncrementInt (Variables|Default|GetGear)
      (:%20%20
        (CallFunction|GetRatio)))))

(event Custom|ShiftGearDown
  (if (and (> (Variables|Default|GetGear) -1) (Variables|Default|GetInGear))
    (Variables|Default|SetInGear false)
    (Variables|Default|SetRatio 0.0)
    (Variables|Default|SetGearText "--")
    (Utilities|FlowControl|Delay (Variables|Default|GetGearShiftTime))
    (Variables|Default|SetInGear true)
    (Math|Integer|DecrementInt (Variables|Default|GetGear)
      (:%20%20
        (CallFunction|GetRatio)))))

(event EventBeginPlay)

(event EventTick
  (params (DeltaSeconds :type Float%20%28single-precision%29)))

(fn GetOutputTorque
  (params (InputTorque :type Float%20%28single-precision%29))
  (return (* InputTorque (Variables|Default|GetRatio))))

(fn GetInputShaftVelocity
  (params (OutputShaftTorque :type Float%20%28single-precision%29))
  (return (* OutputShaftTorque (Variables|Default|GetRatio))))

(fn GetRatio
  (bind _gear (Variables|Default|GetGear))
  (Variables|Default|SetRatio (select (== _gear -1) (Variables|Default|GetReverseGear) (Utilities|Array|Get(acopy) (Variables|Default|GetGearRatio) (Variables|Default|GetGear))))
  (Variables|Default|SetGearText (select (== _gear -1) "R" (Utilities|Select :Index _gear :Option%200 "N" :Option%201 "1" :Option%202 "2" :Option%203 "3" :Option%204 "4" :Option%205 "5" :Option%206 "6" :Option%207 "7"))))