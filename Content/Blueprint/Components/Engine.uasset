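; Engine component that simulates engine RPM and effective torque from throttle input, apparently for vehicle physics.
; BeginPlay caches RPM and rad/s conversion factors, and an externally called UpdatePhysic passes in delta time and throttle to drive the simulation.
; Throttle scales curve torque plus RPM-dependent friction, then friction is subtracted.
; The resulting torque over inertia integrates angular velocity, clamped between idle and max RPM.
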(event Custom|UpdatePhysic
  (params (DeltaTime :type Float%20%28single-precision%29) (Throttle :type Float%20%28single-precision%29))
  (Variables|Default|SetDeltaTime DeltaTime)
  (Variables|Default|SetThrottle Throttle)
  (CallFunction|EngineAcceleration))

(event EventBeginPlay
  (CallFunction|Initialization))

(event EventTick
  (params (DeltaSeconds :type Float%20%28single-precision%29)))

(fn EngineAcceleration
  (bind _rpmtorad (Variables|Math|GetRPMToRad))
  (Variables|Default|SetEngineEffectiveTorque (- (* (+ (Math|Curves|GetFloatValue (Variables|Default|GetEngineTorqueCurve) (Variables|Default|GetEngineRPM)) (+ (Variables|Default|GetStartFriction) (* (Variables|Default|GetEngineRPM) (Variables|Default|GetFrictionCoeff)))) (Variables|Default|GetThrottle)) (+ (Variables|Default|GetStartFriction) (* (Variables|Default|GetEngineRPM) (Variables|Default|GetFrictionCoeff)))))
  (bind _output_get (Variables|Default|SetEngineAngularVelocity (Math|Float|Clamp(Float) (+ (Variables|Default|GetEngineAngularVelocity) (* (/ (- (* (+ (Math|Curves|GetFloatValue (Variables|Default|GetEngineTorqueCurve) (Variables|Default|GetEngineRPM)) (+ (Variables|Default|GetStartFriction) (* (Variables|Default|GetEngineRPM) (Variables|Default|GetFrictionCoeff)))) (Variables|Default|GetThrottle)) (+ (Variables|Default|GetStartFriction) (* (Variables|Default|GetEngineRPM) (Variables|Default|GetFrictionCoeff)))) (Variables|Default|GetEngineInertia)) (Variables|Default|GetDeltaTime))) (* (Variables|Default|GetEngineIdleRPM) _rpmtorad) (* _rpmtorad (Variables|Default|GetEngineMaxRPM)))))
  (Variables|Default|SetEngineRPM (* _output_get (Variables|Math|GetRadToRPM))))

(fn Initialization
  (bind _output_get (Variables|Math|SetRPMToRad (/ (* (Math|Trig|GetPI) 2.0) 6e+01)))
  (Variables|Math|SetRadToRPM (/ 1.0 _output_get)))