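; Drivable rear-wheel-drive car with a component-based drivetrain simulation, chase camera and on-screen debug telemetry.
; Each Tick passes clutch torque through gearbox and differential to the rear wheels, then returns wheel speeds upstream to update clutch and engine.
; Interpolated inputs drive throttle, front steering and biased brakes with rear handbrake; keys shift gears.
; Wheel meshes, created in the construction script, follow suspension length and spin with wheel velocity.
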(event EventBeginPlay
  (Default|Initialize (Variables|Default|GetWheel_FL) (Variables|Default|GetBody)))

(event EventTick
  (params (DeltaSeconds :type Float%20%28single-precision%29))
  (bind _gearbox (Variables|Default|GetGearbox))
  (bind _braketorque (Variables|Brake|GetBrakeTorque))
  (bind _body (Variables|Default|GetBody))
  (bind _engine (Variables|Default|GetEngine))
  (bind _output (Utilities|Array|Get(acopy) _braketorque))
  (bind _output_2 (Utilities|Array|Get(acopy) _braketorque 1))
  (Variables|Default|SetDeltaTime DeltaSeconds)
  (CallFunction|CameraControl)
  (bind _outputtorque (Default|GetOutputTorque (Variables|Default|GetGearbox) (Variables|/Game/Blueprint/Components/Clutch.Clutch_C|GetClutchTorque (Variables|Default|GetClutch))))
  (bind (_outputtorqueleft _outputtorqueright) (Default|GetOutputTorque (Variables|Default|GetDifferential) _outputtorque))
  (Default|UpdatePhysic (Variables|Default|GetWheel_FL) (Variables|Default|GetDeltaTime) 0.0 _output)
  (Default|UpdatePhysic (Variables|Default|GetWheel_FR) (Variables|Default|GetDeltaTime) 0.0 _output)
  (Default|UpdatePhysic (Variables|Default|GetWheel_RL) (Variables|Default|GetDeltaTime) _outputtorqueleft _output_2)
  (Default|UpdatePhysic (Variables|Default|GetWheel_RR) (Variables|Default|GetDeltaTime) _outputtorqueright _output_2)
  (bind _inputshaftvelocity (Default|GetInputShaftVelocity (Variables|Default|GetDifferential) (Variables|/Game/Blueprint/Components/Wheel.Wheel_C|GetWheelAngularVelocity (Variables|Default|GetWheel_RL)) (Variables|/Game/Blueprint/Components/Wheel.Wheel_C|GetWheelAngularVelocity (Variables|Default|GetWheel_RR))))
  (bind _inputshaftvelocity_2 (Default|GetInputShaftVelocity (Variables|Default|GetGearbox) _inputshaftvelocity))
  (Default|UpdatePhysic (Variables|Default|GetClutch) _inputshaftvelocity_2 (Variables|/Game/Blueprint/Components/Engine.Engine_C|GetEngineAngularVelocity (Variables|Default|GetEngine)) (Variables|/Game/Blueprint/Components/Gearbox.Gearbox_C|GetRatio (Variables|Default|GetGearbox)))
  (Default|UpdatePhysic (Variables|Default|GetEngine) (Variables|Default|GetDeltaTime) (Variables|Input|GetThrottle) (Variables|/Game/Blueprint/Components/Clutch.Clutch_C|GetClutchTorque (Variables|Default|GetClutch)))
  (CallFunction|UpdateWheelMesh)
  (Development|PrintString (Utilities|String|Append "EngineRPM = " (Utilities|String|ToString(Float) (Variables|/Game/Blueprint/Components/Engine.Engine_C|GetEngineRPM _engine))) true false "(R=0.000000,G=0.660000,B=1.000000,A=1.000000)" 0.0)
  (Development|PrintString (Utilities|String|Append "Engine Torque = " (Utilities|String|ToString(Float) (Variables|/Game/Blueprint/Components/Engine.Engine_C|GetEngineEffectiveTorque _engine))) true false "(R=0.000000,G=0.660000,B=1.000000,A=1.000000)" 0.0)
  (Development|PrintString (Utilities|String|Append "Gear = " (Utilities|String|ToString(Text) (Variables|/Game/Blueprint/Components/Gearbox.Gearbox_C|GetGearText _gearbox))) true false "(R=0.001821,G=1.000000,B=0.109462,A=1.000000)" 0.0)
  (Development|PrintString (Utilities|String|Append "GearboxRatio = " (Utilities|String|ToString(Float) (Variables|/Game/Blueprint/Components/Gearbox.Gearbox_C|GetRatio _gearbox))) true false "(R=0.001821,G=1.000000,B=0.109462,A=1.000000)" 0.0)
  (Development|PrintString (Utilities|String|Append "Clutch Lock = " (Utilities|String|ToString(Float) (Variables|/Game/Blueprint/Components/Clutch.Clutch_C|GetClutchLock (Variables|Default|GetClutch)))) true true "(R=1.000000,G=0.892658,B=0.062500,A=1.000000)" 0.0)
  (Development|PrintString (Utilities|String|Append "Clutch Torque = " (Utilities|String|ToString(Float) (Variables|/Game/Blueprint/Components/Clutch.Clutch_C|GetClutchTorque (Variables|Default|GetClutch)))) true true "(R=1.000000,G=0.892658,B=0.062500,A=1.000000)" 0.0)
  (bind _returnvalue (Physics|GetPhysicsLinearVelocity _body "None"))
  (Development|PrintString (Utilities|String|Append "speed = " (Utilities|String|ToString(Integer) (Math|Float|Round (* (Math|Vector|DotProduct (Math|Vector|GetForwardVector _body) _returnvalue) 0.036))) " km/h") true false "(R=0.000000,G=0.660000,B=1.000000,A=1.000000)" 0.0))

(event Input|AxisEvents|InputAxisSteering
  (params (AxisValue :type Float%20%28single-precision%29))
  (bind _steeranglenormalized (CallFunction|SteeringInterp AxisValue))
  (Transformation|SetRelativeRotation (Variables|Default|GetSteeringWheel) (Math|Rotator|MakeRotator (* _steeranglenormalized 2.2e+02) -2e+01 0.0) false false))

(event Input|AxisEvents|InputAxisForward
  (params (AxisValue :type Float%20%28single-precision%29)))

(event Input|AxisEvents|InputAxisThrottle
  (params (AxisValue :type Float%20%28single-precision%29))
  (bind _output_get (Variables|Input|SetThrottle (Math|Interpolation|FInterpTo (Variables|Input|GetThrottle) AxisValue (Variables|Default|GetDeltaTime) (select (== AxisValue 0.0) 8.0 4.0))))
  (Development|PrintString (Utilities|String|Append "Throttle = " (Utilities|String|ToString(Float) _output_get)) true false "(R=0.103198,G=1.000000,B=0.114191,A=1.000000)" 0.0))

(event Input|AxisEvents|InputAxisBrake
  (params (AxisValue :type Float%20%28single-precision%29))
  (bind _braketorque (Variables|Brake|GetBrakeTorque))
  (bind _maxbraketorque (Variables|Brake|GetMaxBrakeTorque))
  (bind _brakebias (Variables|Brake|GetBrakeBias))
  (bind _maxbraketorque_2 (Variables|Brake|GetMaxBrakeTorque))
  (bind _output_get (Variables|Input|SetBrake (Math|Interpolation|FInterptoConstant (Variables|Input|GetBrake) AxisValue (Variables|Default|GetDeltaTime) (Math|Float|SelectFloat 8.0 16.0 (!= AxisValue 0.0)))))
  (Development|PrintString (Utilities|String|Append "Brake = " (Utilities|String|ToString(Float) _output_get)) true false "(R=0.103198,G=1.000000,B=0.114191,A=1.000000)" 0.0)
  (Utilities|Array|SetArrayElem _braketorque 0 (* _maxbraketorque (Variables|Input|GetBrake) _brakebias))
  (Utilities|Array|SetArrayElem _braketorque 1 (Math|Float|Min(Float) (+ (* _maxbraketorque (Variables|Input|GetBrake) (- 1.0 _brakebias)) (* (Input|AxisValues|GetHandbrake) _maxbraketorque_2)) _maxbraketorque_2)))

(event Input|KeyboardEvents|L
  (params (Key :type Key%20Structure))
  ;[1 1 1] Shift Gear
  (:Pressed
    (Default|ShiftGearDown (Variables|Default|GetGearbox))))

(event Input|KeyboardEvents|P
  (params (Key :type Key%20Structure))
  ;[1 1 1] Shift Gear
  (:Pressed
    (Default|ShiftGearUp (Variables|Default|GetGearbox))))

(fn ConstructionScript
  (for _index (range 0 3)
    (bind _returnvalue (AddComponent|AddStaticMeshComponent false))
    (Components|StaticMesh|SetStaticMesh _returnvalue (Variables|Wheel|GetWheelMesh))
    (Collision|SetCollisionEnabled _returnvalue "NoCollision")
    (Transformation|SetRelativeScale3D _returnvalue (Math|Vector|MakeVector 1.0 (Utilities|Select :Index _index :Option%200 -1.0 :Option%201 1.0 :Option%202 -1.0 :Option%203 1.0) 1.0))
    (Transformation|SetRelativeLocation _returnvalue (Math|Vector|MakeVector 0.0 0.0 (* (Variables|/Game/Blueprint/Components/Wheel.Wheel_C|GetRestLength (Utilities|Select :Index _index :Option%200 (Variables|Default|GetWheel_FL) :Option%201 (Variables|Default|GetWheel_FR) :Option%202 (Variables|Default|GetWheel_RL) :Option%203 (Variables|Default|GetWheel_RR))) -1.0)) false false)
    (Transformation|AttachComponentToComponent _returnvalue (Utilities|Select :Index _index :Option%200 (Variables|Default|GetWheel_FL) :Option%201 (Variables|Default|GetWheel_FR) :Option%202 (Variables|Default|GetWheel_RL) :Option%203 (Variables|Default|GetWheel_RR)) "None" "KeepRelative" "KeepRelative" "KeepRelative" true)))

(fn CameraControl
  (bind _springarm_chase (Variables|Default|GetSpringArm_Chase))
  (bind _relativerotation (Variables|/Script/Engine.SceneComponent|GetRelativeRotation _springarm_chase))
  (bind (_roll _pitch _yaw) (Math|Rotator|BreakRotator _relativerotation))
  (Transformation|SetRelativeRotation _springarm_chase (Math|Rotator|MakeRotator _roll (Math|Float|Clamp(Float) (+ (Class|Actor|GetInputAxisKeyValue) _pitch) -7e+01 7e+01) (+ _yaw (Class|Actor|GetInputAxisKeyValue))) false false))

(fn UpdateWheelMesh
  (for _index (range 0 3)
    (Transformation|SetRelativeLocation (Components|GetChildComponent (Utilities|Select :Index _index :Option%200 (Variables|Default|GetWheel_FL) :Option%201 (Variables|Default|GetWheel_FR) :Option%202 (Variables|Default|GetWheel_RL) :Option%203 (Variables|Default|GetWheel_RR)) 0) (Math|Vector|MakeVector 0.0 0.0 (* (Variables|/Game/Blueprint/Components/Wheel.Wheel_C|GetCurrentLength (Utilities|Select :Index _index :Option%200 (Variables|Default|GetWheel_FL) :Option%201 (Variables|Default|GetWheel_FR) :Option%202 (Variables|Default|GetWheel_RL) :Option%203 (Variables|Default|GetWheel_RR))) -1.0)) false false)
    (Transformation|AddLocalRotation (Components|GetChildComponent (Utilities|Select :Index _index :Option%200 (Variables|Default|GetWheel_FL) :Option%201 (Variables|Default|GetWheel_FR) :Option%202 (Variables|Default|GetWheel_RL) :Option%203 (Variables|Default|GetWheel_RR)) 0) (Math|Rotator|MakeRotator 0.0 (* (Math|Trig|RadiansToDegrees (Variables|/Game/Blueprint/Components/Wheel.Wheel_C|GetWheelAngularVelocity (Utilities|Select :Index _index :Option%200 (Variables|Default|GetWheel_FL) :Option%201 (Variables|Default|GetWheel_FR) :Option%202 (Variables|Default|GetWheel_RL) :Option%203 (Variables|Default|GetWheel_RR)))) (Variables|Default|GetDeltaTime) -1.0) 0.0) false false)))

(fn SteeringInterp
  (params (Axis :type Float%20%28single-precision%29))
  (bind _deltatime (Variables|Default|GetDeltaTime))
  (bind _output_get (Variables|Input|SetSteeringAngle (Math|Interpolation|FInterpTo (Variables|Input|GetSteeringAngle) (* Axis (Variables|Default|GetMaxSteeringAngle)) _deltatime (* (/ 1.0 _deltatime) (select (== Axis 0.0) 0.3 0.04)))))
  (Transformation|SetRelativeRotation (Variables|Default|GetWheel_FL) (Math|Rotator|MakeRotator 0.0 0.0 _output_get) false false)
  (return (/ (Variables|Input|GetSteeringAngle) (Variables|Default|GetMaxSteeringAngle))))